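; Base tile actor for infinite terrain, with a barrier wall and an arrow that supplies an attach transform.
; The barrier starts locked, turns non-colliding translucent green while the player is inside the area volume, and returns to solid red collision on leaving.
; Leaving the area also asks InfinteTerrainGameMode to spawn a tile.
; The player entering the exit volume destroys the tile.
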(event OnComponentEndOverlap(AreaBoundsVolume)
  (params (OverlappedComponent :type Primitive%20Component%20Object%20Reference) (OtherActor :type Actor%20Object%20Reference) (OtherComp :type Primitive%20Component%20Object%20Reference) (OtherBodyIndex :type Integer))
  (Utilities|IsPlayerActor OtherActor
    (:True
      (CallFunction|LockBarrierWall)
      (bind _asinfinte_terrain_game_mode (Utilities|Casting|CastToInfinteTerrainGameMode (Game|GetGameMode)))
      (Default|SpawnTile _asinfinte_terrain_game_mode))))

(event OnComponentBeginOverlap(AreaBoundsVolume)
  (params (OverlappedComponent :type Primitive%20Component%20Object%20Reference) (OtherActor :type Actor%20Object%20Reference) (OtherComp :type Primitive%20Component%20Object%20Reference) (OtherBodyIndex :type Integer) (bFromSweep :type Boolean) (SweepResult :type Hit%20Result%20Structure%20%28by%20ref%29))
  (Utilities|IsPlayerActor OtherActor
    (:True
      (CallFunction|UnlockBarrierWall))))

(event OnComponentBeginOverlap(ExitBoundsVolume)
  (params (OverlappedComponent :type Primitive%20Component%20Object%20Reference) (OtherActor :type Actor%20Object%20Reference) (OtherComp :type Primitive%20Component%20Object%20Reference) (OtherBodyIndex :type Integer) (bFromSweep :type Boolean) (SweepResult :type Hit%20Result%20Structure%20%28by%20ref%29))
  (Utilities|IsPlayerActor OtherActor
    (:True
      (Actor|DestroyActor)
      (Development|PrintString "Destroyed Tile by Exit"))))

(event EventBeginPlay
  (CallFunction|LockBarrierWall))

(fn ConstructionScript)

(fn GetTileAttachTransform
  (return (Transformation|GetWorldTransform (Variables|Default|GetLocateArrow))))

(fn LockBarrierWall
  (bind _staticmesh_barrierwall (Variables|Default|GetStaticMesh_BarrierWall))
  (Collision|SetCollisionEnabled _staticmesh_barrierwall "QueryAndPhysics")
  (Development|PrintString "Barrier Locked")
  (Rendering|Material|SetMaterial _staticmesh_barrierwall 0 "/Game/Static/Geometry/Meshes/BarrierRedSolid.BarrierRedSolid"))

(fn UnlockBarrierWall
  (bind _staticmesh_barrierwall (Variables|Default|GetStaticMesh_BarrierWall))
  (Collision|SetCollisionEnabled _staticmesh_barrierwall "NoCollision")
  (Development|PrintString "Barrier Unlocked")
  (Rendering|Material|SetMaterial _staticmesh_barrierwall 0 "/Game/Static/Geometry/Meshes/BarrierGreenTrans.BarrierGreenTrans"))