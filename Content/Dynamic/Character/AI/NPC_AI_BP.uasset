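; AI controller for guard NPCs that spots non-guard actors and makes the guard aim.
; On BeginPlay it initializes the PatrolData blackboard and runs the GuardBehavior tree.
; Perception updates ignore actors tagged Guard, set FocusActor on sensing and clear it on any loss, toggling IsAiming on the controlled PlayerGuardCharacter to match.
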(event OnTargetPerceptionUpdated(AIPerception)
  (params (Actor :type Actor%20Object%20Reference) (Stimulus :type AI%20Stimulus%20Structure))
  (bind _returnvalue (Utilities|String|StringToName "FocusActor"))
  (bind _self self)
  (bind _blackboardref (Variables|Default|GetBlackboardRef))
  (bind _returnvalue_2 (Pawn|GetControlledPawn _self))
  (if (not (Actor|ActorHasTag Actor "Guard"))
    (if (.bSuccessfullySensed (Utilities|Struct|BreakAIStimulus Stimulus))
      (AI|Components|Blackboard|SetValueasObject _blackboardref _returnvalue Actor)
      (bind _asplayer_guard_character (Utilities|Casting|CastToPlayerGuardCharacter _returnvalue_2))
      (Variables|/Game/Dynamic/Character/PlayerGuardCharacter.PlayerGuardCharacter_C|SetIsAiming _asplayer_guard_character true)
      (else
        (AI|Components|Blackboard|ClearValue _blackboardref _returnvalue)
        (bind _asplayer_guard_character_2 (Utilities|Casting|CastToPlayerGuardCharacter _returnvalue_2))
        (Variables|/Game/Dynamic/Character/PlayerGuardCharacter.PlayerGuardCharacter_C|SetIsAiming _asplayer_guard_character_2 false)))))

(event EventBeginPlay
  (bind _blackboardcomponent (Class|AIController|UseBlackboard "/Game/Dynamic/Character/AI/PatrolData.PatrolData"))
  (Variables|Default|SetBlackboardRef _blackboardcomponent)
  (AI|RunBehaviorTree "/Game/Dynamic/Character/AI/GuardBehavior.GuardBehavior"))

(fn ConstructionScript)